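; Rule set that fakes environmental gunshot echoes for the first player's weapons, binding to each inventory weapon's fire event on spawn.
; Each shot plays a thump and sends nine world-static line traces along horizontal offsets from the aim direction.
; Each hit plays a reverb sound at the impact after a round-trip speed-of-sound delay from the player, with pitch falling as that delay grows and volume derived from trace distance.
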(event Custom|OnFired
  (params (FiredWeapon :type DF%20Base%20Weapon%20Object%20Reference) (bLastFire :type Boolean))
  (Utilities|FlowControl|Sequence
    (:then_0
      (Utilities|CreateReverb FiredWeapon "-1.000000,1.000000,0.000000"))
    (:then_1
      (Utilities|CreateReverb FiredWeapon "0,1.000000,0"))
    (:then_2
      (Utilities|CreateReverb FiredWeapon "1.000000,1.000000,0"))
    (:then_3
      (Utilities|CreateReverb FiredWeapon "-1.000000,0,0"))
    (:then_4
      (Utilities|CreateReverb FiredWeapon))
    (:then_5
      (Utilities|CreateReverb FiredWeapon "1.000000,0,0"))
    (:then_6
      (Utilities|CreateReverb FiredWeapon "-1.000000,-1.000000,0"))
    (:then_7
      (Utilities|CreateReverb FiredWeapon "0,-1.000000,0"))
    (:then_8
      (Utilities|CreateReverb FiredWeapon "1.000000,-1.000000,0"))
    (:then_9
      (Audio|PlaySoundatLocation "/XorberaxReverb/Core/Audio/SND_Thump_Cue.SND_Thump_Cue" (Transformation|GetActorLocation FiredWeapon) "0, 0, 0" 1.0 1.0 0.0 0 0 FiredWeapon))))

(event EventPlayerSpawn
  (params (Player :type Controller%20Object%20Reference) (NewPlayerPawn :type Pawn%20Object%20Reference))
  (if (== Player (Game|GetPlayerController 0)) ; Connect this node to only apply reverb to player.
    (bind _ashdplayer_character (Utilities|Casting|CastToHDPlayerCharacter NewPlayerPawn))
    (for _array_element (Variables|/Script/DonkehFramework.DFInventoryComponent|GetItems (Variables|/Script/DonkehFramework.DFBaseCharacter|GetInventory _ashdplayer_character))
      (bind _asbp_hdweapon_base (Utilities|Casting|CastToBP_HDWeaponBase _array_element))
      (EventDispatchers|BindEventtoOnFire _asbp_hdweapon_base (delegate Custom|OnFired)))))