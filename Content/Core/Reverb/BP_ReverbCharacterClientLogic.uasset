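; Client-side gunshot reverb logic that binds to OnFire on the replicated character's inventory weapons.
; Each supported shot casts jittered world-static traces in eleven directions and queues echoes at hit points, choosing cue, volume and pitch by distance, plus a bass thump for the local shooter.
; Tick plays echoes once world time reaches TriggerTime, which holds only the player-to-hit round-trip sound delay, without current time added.
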(event Collision|EventActorBeginOverlap
  (params (OtherActor :type Actor%20Object%20Reference)))

(event Custom|OnFire
  (params (FiredWeapon :type DF%20Base%20Weapon%20Object%20Reference) (bLastFire :type Boolean))
  (bind _returnvalue (Class|DFBaseItem|GetItemType FiredWeapon))
  (bind (_weaponreverbconfig _issupported) (CallFunction|GetWeaponReverbConfig _returnvalue))
  (bind (_volumemultiplier _pitchmultiplier _distancemultiplier _thumpvolume _thumppitch) (Utilities|Struct|BreakWeaponReverbConfig _weaponreverbconfig))
  ;[1 1 1] Handle Weapon Fire Event
  (if (not (and (CallFunction|IsClient) (Class|DFBlueprintFunctions|IsPendingKillPending FiredWeapon)))
    (bind _asdfbase_gun (Utilities|Casting|CastToDFBaseGun FiredWeapon))
    (if _issupported
      (Utilities|FlowControl|Sequence
        (:then_0
          ;;[1 1 1] Environmental Reverb
          (Utilities|CreateReverb FiredWeapon "0,0,1.000000" (Class|DFBaseGun|GetMuzzleLocation _asdfbase_gun false) (Class|DFBaseGun|GetMuzzleDirection _asdfbase_gun false) _weaponreverbconfig))
        (:then_1
          (Utilities|CreateReverb FiredWeapon "-1.000000,1.000000,0" (Class|DFBaseGun|GetMuzzleLocation _asdfbase_gun false) (Class|DFBaseGun|GetMuzzleDirection _asdfbase_gun false) _weaponreverbconfig))
        (:then_2
          (Utilities|CreateReverb FiredWeapon "0,1.000000,0" (Class|DFBaseGun|GetMuzzleLocation _asdfbase_gun false) (Class|DFBaseGun|GetMuzzleDirection _asdfbase_gun false) _weaponreverbconfig))
        (:then_3
          (Utilities|CreateReverb FiredWeapon "1.000000,1.000000,0" (Class|DFBaseGun|GetMuzzleLocation _asdfbase_gun false) (Class|DFBaseGun|GetMuzzleDirection _asdfbase_gun false) _weaponreverbconfig))
        (:then_4
          (Utilities|CreateReverb FiredWeapon "-1.000000,0,0" (Class|DFBaseGun|GetMuzzleLocation _asdfbase_gun false) (Class|DFBaseGun|GetMuzzleDirection _asdfbase_gun false) _weaponreverbconfig))
        (:then_5
          (Utilities|CreateReverb :Weapon FiredWeapon :MuzzleLocation (Class|DFBaseGun|GetMuzzleLocation _asdfbase_gun false) :MuzzleDirection (Class|DFBaseGun|GetMuzzleDirection _asdfbase_gun false) :WeaponReverbConfig _weaponreverbconfig))
        (:then_6
          (Utilities|CreateReverb FiredWeapon "1.000000,0,0" (Class|DFBaseGun|GetMuzzleLocation _asdfbase_gun false) (Class|DFBaseGun|GetMuzzleDirection _asdfbase_gun false) _weaponreverbconfig))
        (:then_7
          (Utilities|CreateReverb FiredWeapon "-1.000000,-1.000000,0" (Class|DFBaseGun|GetMuzzleLocation _asdfbase_gun false) (Class|DFBaseGun|GetMuzzleDirection _asdfbase_gun false) _weaponreverbconfig))
        (:then_8
          (Utilities|CreateReverb FiredWeapon "0,-1.000000,0" (Class|DFBaseGun|GetMuzzleLocation _asdfbase_gun false) (Class|DFBaseGun|GetMuzzleDirection _asdfbase_gun false) _weaponreverbconfig))
        (:then_9
          (Utilities|CreateReverb FiredWeapon "1.000000,-1.000000,0" (Class|DFBaseGun|GetMuzzleLocation _asdfbase_gun false) (Class|DFBaseGun|GetMuzzleDirection _asdfbase_gun false) _weaponreverbconfig))
        (:then_10
          (Utilities|CreateReverb FiredWeapon "0,0,-1.000000" (Class|DFBaseGun|GetMuzzleLocation _asdfbase_gun false) (Class|DFBaseGun|GetMuzzleDirection _asdfbase_gun false) _weaponreverbconfig))
        (:then_11
          ;;[1 1 1] Firing Thump/Bass Boost
          (if (== (Pawn|GetController (Variables|/Script/DonkehFramework.DFBaseItem|GetPawnOwner FiredWeapon)) (Game|GetPlayerController 0)) ; Check if shooter is player
            (Audio|PlaySoundatLocation "/XorberaxReverb/Core/Reverb/Audio/SND_Thump_Cue.SND_Thump_Cue" (Transformation|GetActorLocation FiredWeapon) "0, 0, 0" _thumpvolume _thumppitch 0.0 0 0 FiredWeapon)))))))

(event EventTick
  (params (DeltaSeconds :type Float%20%28single-precision%29))
  (bind _queuedreverbevents (Variables|Default|GetQueuedReverbEvents))
  (if (CallFunction|IsClient)
    (for (_array_element _array_index) _queuedreverbevents
      (if (>= (Utilities|Time|GetTimeSeconds) (.triggertime _array_element))
        (Audio|PlaySoundatLocation (.reverbsoundcue _array_element) (.location _array_element) "0, 0, 0" (.volumemultiplier _array_element) (.pitchmultiplier _array_element) 0.0 0 0 (.owner _array_element))
        (Utilities|Array|RemoveIndex _queuedreverbevents _array_index)))))

(fn ConstructionScript)

(fn OnRepCharacter
  (for _array_element (Variables|/Script/DonkehFramework.DFInventoryComponent|GetItems (Variables|/Script/DonkehFramework.DFBaseCharacter|GetInventory (Variables|Default|GetCharacter)))
    (bind _asbp_hdweapon_base (Utilities|Casting|CastToBP_HDWeaponBase _array_element))
    (EventDispatchers|BindEventtoOnFire _asbp_hdweapon_base (EventDispatchers|CreateEvent :!event Custom|OnFire))))

(fn IsClient
  (bind _returnvalue (Ability|HasAuthority))
  (bind _returnvalue_2 (Networking|IsDedicatedServer))
  (bind _returnvalue_3 (not _returnvalue_2))
  (return (or (and (not _returnvalue) _returnvalue_3) (and _returnvalue _returnvalue_3))))

(fn GetWeaponReverbConfig
  (params (WeaponType :type EItemType%20Enum :default "Melee"))
  (bind _weaponreverbconfigs (Variables|Default|GetWeaponReverbConfigs))
  (bind (_value _returnvalue) (Utilities|Map|Find _weaponreverbconfigs WeaponType))
  (return _value _returnvalue))

(fn GetReverbSoundCue
  (params (Distance :type Float%20%28single-precision%29))
  (if (< Distance 1e+03)
    (return "/XorberaxReverb/Core/Reverb/Audio/SND_ReverbClose_Cue.SND_ReverbClose_Cue")
    (elif (< Distance 7e+03)
      (return "/XorberaxReverb/Core/Reverb/Audio/SND_ReverbMid_Cue.SND_ReverbMid_Cue")
      (else
        (return "/XorberaxReverb/Core/Reverb/Audio/SND_ReverbFar_Cue.SND_ReverbFar_Cue")))))