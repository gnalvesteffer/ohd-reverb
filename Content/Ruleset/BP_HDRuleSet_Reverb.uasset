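; Ruleset that fakes environmental gunfire reverb, binding to the fire event of weapons in each spawned character's inventory.
; Each supported shot sends eleven jittered static-world traces around the muzzle direction, playing echoes at impacts after a delay based on listener distance and sound speed.
; Per-weapon config scales volume and pitch, and player 0's shots add a bass thump.
; The far cue is unreachable due to a constant comparison, and the player-only filter is disconnected.
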(event Custom|OnFire
  (params (FiredWeapon :type DF%20Base%20Weapon%20Object%20Reference) (bLastFire :type Boolean))
  (bind _returnvalue (Class|DFBaseItem|GetItemType FiredWeapon))
  (bind (_weaponreverbconfig _issupported) (CallFunction|GetWeaponReverbConfig _returnvalue))
  (bind (_volumemultiplier _pitchmultiplier _distancemultiplier _thumpvolume _thumppitch) (Utilities|Struct|BreakWeaponReverbConfig _weaponreverbconfig))
  ;[1 1 1] Handle Weapon Fire Event
  (bind _asdfbase_gun (Utilities|Casting|CastToDFBaseGun FiredWeapon))
  (if _issupported
    (Utilities|FlowControl|Sequence
      (:then_0
        ;;[1 1 1] Environmental Reverb
        (Utilities|CreateReverb FiredWeapon "-1.000000,1.000000,0.000000" (Class|DFBaseGun|GetMuzzleLocation _asdfbase_gun false) (Class|DFBaseGun|GetMuzzleDirection _asdfbase_gun false) _weaponreverbconfig))
      (:then_1
        (Utilities|CreateReverb FiredWeapon "0,1.000000,0" (Class|DFBaseGun|GetMuzzleLocation _asdfbase_gun false) (Class|DFBaseGun|GetMuzzleDirection _asdfbase_gun false) _weaponreverbconfig))
      (:then_2
        (Utilities|CreateReverb FiredWeapon "1.000000,1.000000,0" (Class|DFBaseGun|GetMuzzleLocation _asdfbase_gun false) (Class|DFBaseGun|GetMuzzleDirection _asdfbase_gun false) _weaponreverbconfig))
      (:then_3
        (Utilities|CreateReverb FiredWeapon "-1.000000,0,0" (Class|DFBaseGun|GetMuzzleLocation _asdfbase_gun false) (Class|DFBaseGun|GetMuzzleDirection _asdfbase_gun false) _weaponreverbconfig))
      (:then_4
        (Utilities|CreateReverb :Weapon FiredWeapon :MuzzleLocation (Class|DFBaseGun|GetMuzzleLocation _asdfbase_gun false) :MuzzleDirection (Class|DFBaseGun|GetMuzzleDirection _asdfbase_gun false) :WeaponReverbConfig _weaponreverbconfig))
      (:then_5
        (Utilities|CreateReverb FiredWeapon "1.000000,0,0" (Class|DFBaseGun|GetMuzzleLocation _asdfbase_gun false) (Class|DFBaseGun|GetMuzzleDirection _asdfbase_gun false) _weaponreverbconfig))
      (:then_6
        (Utilities|CreateReverb FiredWeapon "-1.000000,-1.000000,0" (Class|DFBaseGun|GetMuzzleLocation _asdfbase_gun false) (Class|DFBaseGun|GetMuzzleDirection _asdfbase_gun false) _weaponreverbconfig))
      (:then_7
        (Utilities|CreateReverb FiredWeapon "0,-1.000000,0" (Class|DFBaseGun|GetMuzzleLocation _asdfbase_gun false) (Class|DFBaseGun|GetMuzzleDirection _asdfbase_gun false) _weaponreverbconfig))
      (:then_8
        (Utilities|CreateReverb FiredWeapon "1.000000,-1.000000,0" (Class|DFBaseGun|GetMuzzleLocation _asdfbase_gun false) (Class|DFBaseGun|GetMuzzleDirection _asdfbase_gun false) _weaponreverbconfig))
      (:then_9
        (Utilities|CreateReverb FiredWeapon "0,0.000000,1.000000" (Class|DFBaseGun|GetMuzzleLocation _asdfbase_gun false) (Class|DFBaseGun|GetMuzzleDirection _asdfbase_gun false) _weaponreverbconfig))
      (:then_10
        (Utilities|CreateReverb FiredWeapon "0,0.000000,-1.000000" (Class|DFBaseGun|GetMuzzleLocation _asdfbase_gun false) (Class|DFBaseGun|GetMuzzleDirection _asdfbase_gun false) _weaponreverbconfig))
      (:then_11
        ;;[1 1 1] Firing Thump/Bass Boost
        (if (== (Pawn|GetController (Variables|/Script/DonkehFramework.DFBaseItem|GetPawnOwner FiredWeapon)) (Game|GetPlayerController 0)) ; Check if shooter is player
          (Audio|PlaySoundatLocation "/XorberaxReverb/Ruleset/Audio/SND_Thump_Cue.SND_Thump_Cue" (Transformation|GetActorLocation FiredWeapon) "0, 0, 0" _thumpvolume _thumppitch 0.0 0 0 FiredWeapon))))))

(event EventPlayerSpawn
  (params (Player :type Controller%20Object%20Reference) (NewPlayerPawn :type Pawn%20Object%20Reference))
  ;[1 1 1] Bind Weapon Fire Event
  (bind _ashdplayer_character (Utilities|Casting|CastToHDPlayerCharacter NewPlayerPawn))
  (for _array_element (Variables|/Script/DonkehFramework.DFInventoryComponent|GetItems (Variables|/Script/DonkehFramework.DFBaseCharacter|GetInventory _ashdplayer_character))
    (bind _asbp_hdweapon_base (Utilities|Casting|CastToBP_HDWeaponBase _array_element))
    (EventDispatchers|BindEventtoOnFire _asbp_hdweapon_base (delegate Custom|OnFire))))

(fn GetWeaponReverbConfig
  (params (WeaponType :type EItemType%20Enum :default "Melee"))
  (bind _weaponreverbconfigs (Variables|Default|GetWeaponReverbConfigs))
  (bind (_value _returnvalue) (Utilities|Map|Find _weaponreverbconfigs WeaponType))
  (return _value _returnvalue))

(fn GetReverbSoundCue
  (params (DistanceAmount :type Float%20%28single-precision%29))
  (if (< DistanceAmount 0.1)
    (return "/XorberaxReverb/Ruleset/Audio/SND_ReverbClose_Cue.SND_ReverbClose_Cue")
    (elif (< 0.0 0.5)
      (return "/XorberaxReverb/Ruleset/Audio/SND_ReverbMid_Cue.SND_ReverbMid_Cue")
      (else
        (return "/XorberaxReverb/Ruleset/Audio/SND_ReverbFar_Cue.SND_ReverbFar_Cue")))))